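; BP_Goal is a ping-pong goal actor that keeps a score and shows it on a widget.
; The MC_Goal event increments Score, casts its Widget component's user widget to BP_ScoreWidget, and passes the new value through that widget's custom event.
; The Cube's hit and overlap events are empty, so the file itself does no goal detection and relies on MC_Goal being called.
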(event `self.Cube.OnComponentHit`
  (params (HitComponent :type "PrimitiveComponent Object Reference") (OtherActor :type "Actor Object Reference") (OtherComp :type "PrimitiveComponent Object Reference") (NormalImpulse :type "Vector Structure") (Hit :type "HitResult Structure (by ref)")))

(event `self.Cube.OnComponentBeginOverlap`
  (params (OverlappedComponent :type "PrimitiveComponent Object Reference") (OtherActor :type "Actor Object Reference") (OtherComp :type "PrimitiveComponent Object Reference") (OtherBodyIndex :type Integer) (bFromSweep :type Boolean) (SweepResult :type "HitResult Structure (by ref)")))

(event `MC_Goal`
  (set `self.score` (+ (`self.score`) 1))
  (bind _asbp_score_widget (cast `/Game/pingpong/ui/BP_ScoreWidget` (`WidgetComponent.GetWidget` (`self.Widget`))))
  (`/Game/pingpong/ui/BP_ScoreWidget.CustomEvent_0` _asbp_score_widget (`self.score`)))

(fn `UserConstructionScript`)