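; Game mode for the ping pong game that starts play once enough players have joined.
; Each PostLogin calls NewPlayer, which increments a player count.
; When the count exceeds one, it finds the BP_PingPongBall, calls StartMove on it and calls SetStart on the strength widget held by the ball's widget component.
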(event `NewPlayer`
  (set `self.PlayerCount` (+ (`self.PlayerCount`) 1))
  (if (> (`self.PlayerCount`) 1)
    (bind _returnvalue (`GameplayStatics.GetActorOfClass` "/Game/pingpong/bp/BP_PingPongBall.BP_PingPongBall_C"))
    (`PingPongBall.StartMove` _returnvalue)
    (bind _asbp_strength_widget (cast `/Game/pingpong/ui/BP_StrengthWidget` (`WidgetComponent.GetWidget` (`/Game/pingpong/bp/BP_PingPongBall.Widget` _returnvalue))))
    (`/Game/pingpong/ui/BP_StrengthWidget.SetStart` _asbp_strength_widget)))

(event `self.K2_PostLogin`
  (params (NewPlayer :type "PlayerController Object Reference"))
  (`self.NewPlayer`))

(event `self.ReceiveTick`
  (params (DeltaSeconds :type "Float (single-precision)")))

(fn `UserConstructionScript`)