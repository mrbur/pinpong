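; BP_PingPongBall is the ball for the ping pong game, building up a Strength value as it hits things.
; On each body hit against anything but a BP_Goal, it increments Strength and updates its BP_StrengthWidget display.
; Hitting a BP_Goal passes the accumulated Strength to the goal through MCGoal, then empties the widget and resets Strength to zero.
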(event `self.BodyCollision.OnComponentHit`
  (params (HitComponent :type "PrimitiveComponent Object Reference") (OtherActor :type "Actor Object Reference") (OtherComp :type "PrimitiveComponent Object Reference") (NormalImpulse :type "Vector Structure") (Hit :type "HitResult Structure (by ref)"))
  (bind _returnvalue (`WidgetComponent.GetWidget` (`self.Widget`)))
  (bind _asbp_goal (cast `/Game/pingpong/bp/BP_Goal` OtherActor)
    (:`then`
      (`/Game/pingpong/bp/BP_Goal.MC_Goal` _asbp_goal (`self.strength`))
      (bind _asbp_strength_widget (cast `/Game/pingpong/ui/BP_StrengthWidget` _returnvalue))
      (`/Game/pingpong/ui/BP_StrengthWidget.SetEmpty` _asbp_strength_widget)
      (set `self.strength` 0))
    (:`CastFailed`
      (bind _asbp_strength_widget_2 (cast `/Game/pingpong/ui/BP_StrengthWidget` _returnvalue))
      (`/Game/pingpong/ui/BP_StrengthWidget.SetStrenth` _asbp_strength_widget_2 1)
      (set `self.strength` (+ (`self.strength`) 1)))))

(fn `UserConstructionScript`)